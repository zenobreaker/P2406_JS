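; BP_CAttachment_Hammer is the hammer weapon's attachment actor, managing where the hammer mesh sits and when it is visible.
; On BeginPlay it attaches to Hand_Hammer and hides its skeletal mesh.
; Beginning an equip shows the mesh and prints its visibility as debug output, while unequipping reuses the BeginPlay hide step.
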(event EventBeginPlay
  (Class|CAttachment|Attachto "Hand_Hammer")
  (Rendering|SetVisibility (Variables|Default|GetSkeletalMesh) false false))

(event EventOnUnequip
  (Rendering|SetVisibility (Variables|Default|GetSkeletalMesh) false false))

(event EventOnBeginEquip
  (Rendering|SetVisibility (Variables|Default|GetSkeletalMesh) true false)
  (Development|PrintString (Utilities|String|ToString(Boolean) (Rendering|IsVisible (Variables|Default|GetSkeletalMesh)))))

(fn ConstructionScript)