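; BP_CAttachment_Sword2 is the attachment for the Sword2 weapon, moving its mesh between holster and hand.
; On BeginPlay and on unequip it attaches to the Holster_Sword2 socket and hides the static mesh.
; When equipping begins it attaches to Hand_Sword2, shows the mesh and prints the visibility state to the screen.
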(event EventOnBeginEquip
  (Class|CAttachment|Attachto "Hand_Sword2")
  (Rendering|SetVisibility (Variables|Default|GetStaticMesh) true false)
  (Development|PrintString (Utilities|String|ToString(Boolean) (Rendering|IsVisible (Variables|Default|GetStaticMesh)))))

(event EventBeginPlay
  (Class|CAttachment|Attachto "Holster_Sword2")
  (Rendering|SetVisibility (Variables|Default|GetStaticMesh) false false))

(event EventOnUnequip
  (Class|CAttachment|Attachto "Holster_Sword2")
  (Rendering|SetVisibility (Variables|Default|GetStaticMesh) false false))

(fn ConstructionScript)